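; Sample interactable actor that starts a character dialogue when the player interacts with it.
; It picks the tutorial dialogue or a back dialogue using a dot product test of whether the instigator stands in front.
; Interact shows the cached WBP_Dialogue from WidgetCreator, hides the player HUD overlay and switches to UI-only input.
; When the dialogue finishes, it unbinds the event and restores game input and the overlay.
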(event Custom|On%20Finished%20Dialogue
  ;[1 1 1] Giving the control back to the player
  (Input|SetInputModeGameOnly (Game|GetPlayerController 0) false)
  ;[1 1 1] Stop listening for the widget events
  (EventDispatchers|UnbindallEventsfromOnFinishedDialogue (CallFunction|GetDialogueWidget))
  ;[1 1 1] Show back the player overlay
  (Class|CommonHUDSubsystem|SetOverlayLayerVisibility (Subsystems|GetCommonHUDSubsystem (Game|GetPlayerController 0)) "(TagName=\"UI.HudLayout.Overlay.Player\")" "Visible"))

(event EventBeginPlay
  (Class|WidgetCreatorComponent|CreateDefaultWidgets (Variables|Default|GetWidgetCreator)))

(event EventInteract
  (params (InteractionInstigator :type Actor%20Object%20Reference))
  ;[1 1 1] Show the dialogue widget
  (Widget|SetVisibility (CallFunction|GetDialogueWidget) "Visible")
  ;[1 1 1] Hide the player overlay
  (Class|CommonHUDSubsystem|SetOverlayLayerVisibility (Subsystems|GetCommonHUDSubsystem (Game|GetPlayerController 0)) "(TagName=\"UI.HudLayout.Overlay.Player\")" "Collapsed")
  ;[1 1 1] Initializing the dialogue asset for the widget
  (Default|SetDialogueAsset (CallFunction|GetDialogueWidget) (CallFunction|GetDialogueInteraction InteractionInstigator))
  ;[1 1 1] Disabling player controls to interact with the dialogue widget
  (Input|SetInputModeUIOnly (Game|GetPlayerController 0) 0 "DoNotLock" true)
  ;[1 1 1] Start listening to when the dialogue is finished
  (EventDispatchers|AssignOnFinishedDialogue (CallFunction|GetDialogueWidget) (EventDispatchers|CreateEvent :!event Custom|On%20Finished%20Dialogue)))

(fn ConstructionScript)

(fn IsInteractionInstigatorinFront
  (params (Instigator :type Actor%20Object%20Reference))
  (return (>= (Math|Vector|DotProduct (Math|Vector|Normalize (- (Transformation|GetActorLocation Instigator) (Transformation|GetActorLocation))) (Transformation|GetActorForwardVector)) 0.3)))

(fn GetDialogueInteraction
  (params (Interaction%20Instigator :type Actor%20Object%20Reference))
  (if (CallFunction|IsInteractionInstigatorinFront Interaction%20Instigator)
    (return "/Game/Project/Data/Dialogues/DA_Character_TutorialDialogue.DA_Character_TutorialDialogue")
    (else
      (return "/Game/Project/Data/Dialogues/DA_Character_BackDialogue.DA_Character_BackDialogue"))))

(fn GetDialogueWidget
  (bind _aswbp_dialogue (Utilities|Casting|CastToWBP_Dialogue (Class|WidgetCreatorComponent|GetCachedWidgetbyTagChecked (Variables|Default|GetWidgetCreator) "(TagName=\"UI.Widget.DialogueCharacter.Dialogue\")")))
  (return _aswbp_dialogue))

(fn CanInteract
  (params (InteractionInstigator :type Actor%20Object%20Reference))
  (return true))