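; Base Blueprint for collectable items that shows an interaction indicator when an instigator focuses on it.
; On BeginPlay, a WidgetCreator component creates default widgets, and the indicator is fetched from its cache by gameplay tag.
; Focus shows the indicator with collect or full text, depending on whether the instigator's inventory has a free slot; losing focus collapses it.
; CanInteract always returns true, and no pickup logic is defined here.
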(event EventOnUnfocused
  (params (InteractionInstigator :type Actor%20Object%20Reference))
  ;[1 1 1] Hiding the interaction text
  (Widget|SetVisibility (CallFunction|GetInteractionWidget) "Collapsed"))

(event EventOnFocused
  (params (InteractionInstigator :type Actor%20Object%20Reference))
  ;[1 1 1] Updating the interaction text
  (CallFunction|UpdateInteractionText InteractionInstigator)
  ;[1 1 1] Displaying the interaction text
  (Widget|SetVisibility (CallFunction|GetInteractionWidget) "Visible"))

(event EventBeginPlay
  ;[1 1 1] Creating the interaction indicator widget
  (Class|WidgetCreatorComponent|CreateDefaultWidgets (Variables|Default|GetWidgetCreator)))

(fn ConstructionScript)

(fn CanInteract
  (params (InteractionInstigator :type Actor%20Object%20Reference))
  (return true))

(fn GetInteractionWidget
  (bind _aswbp_collectable_indicator (Utilities|Casting|CastToWBP_Collectable_Indicator (Class|WidgetCreatorComponent|GetCachedWidgetbyTagChecked (Variables|Default|GetWidgetCreator) "(TagName=\"UI.Widget.Collectable.Indicator\")")))
  (return _aswbp_collectable_indicator))

(fn UpdateInteractionText
  (params (Instigator :type Actor%20Object%20Reference))
  (bind _returnvalue (Class|InventoryInterface|GetInventoryComponent(Message) Instigator))
  (if (Class|InventoryComponent|HasSlotFree _returnvalue)
    (Default|SetTexttoCollect (CallFunction|GetInteractionWidget))
    (else
      (Default|SetTexttoFull (CallFunction|GetInteractionWidget)))))